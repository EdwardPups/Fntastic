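; BP_Player is the player pawn, handling movement, mouse look and interaction with objects in the world.
; Axis inputs drive movement along the Mesh forward and right vectors and feed controller yaw and pitch.
; The Interaction action fires a short complex Visibility line trace from the Camera, with debug drawing enabled, and sends IntreactionMessage to the hit actor.
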(event `self.ReceiveBeginPlay`)

(event `InputAction|Interaction`
  (params (Key :type "Key Structure"))
  (bind _camera (`self.Camera`))
  (bind _returnvalue (`SceneComponent.K2_GetComponentLocation` _camera))
  (:`Pressed`
    (bind _outhit (`KismetSystemLibrary.LineTraceSingle` :`Start` _returnvalue :`End` (+ _returnvalue (* (`SceneComponent.GetForwardVector` _camera) 1000.0)) :`TraceChannel` "TraceTypeQuery1" :`bTraceComplex` true :`DrawDebugType` "ForDuration"))
    (bind (_bblockinghit _binitialoverlap _time _distance _location _impactpoint _normal _impactnormal _physmat _hitactor) (`GameplayStatics.BreakHitResult` _outhit))
    (if _bblockinghit
      (message `/Game/FntasticTest/Blueprints/Core/Interfaces/BPI_Interaction.Intreaction` _hitactor))))

(event `InputAxis|MovementFB`
  (params (AxisValue :type "Float (single-precision)"))
  (`self.AddMovementInput` (`SceneComponent.GetForwardVector` (`self.Mesh`)) AxisValue))

(event `InputAxis|MovementRL`
  (params (AxisValue :type "Float (single-precision)"))
  (`self.AddMovementInput` (`SceneComponent.GetRightVector` (`self.Mesh`)) AxisValue))

(event `InputAxis|MouseX`
  (params (AxisValue :type "Float (single-precision)"))
  (`self.AddControllerYawInput` AxisValue))

(event `InputAxis|MouseY`
  (params (AxisValue :type "Float (single-precision)"))
  (`self.AddControllerPitchInput` AxisValue))

(fn `UserConstructionScript`)